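; AI character Blueprint that fires an automatic rifle until told to stop or until death.
; StartFireWeapon loops FireAssault on a timer, which StopFireWeapon clears, also bound to the death request.
; Each shot spawns muzzle effect, sound and bullet at an arrow socketed to the gun, provided AmmoInClip exceeds a threshold.
; Spread calculation, fire animation and ammo decrement are disconnected, so shots fly straight without consuming ammo.
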(event `self.ReceiveBeginPlay`
  ;[1 1 1] If the AI dies it will stop them from shooting
  (add `self.AIOnDeathRequest` (delegate `StopFireWeapon`)))

(event `StopFireWeapon`
  ;[1 1 1] If the AI dies it will stop them from shooting
  (`KismetSystemLibrary.K2_ClearAndInvalidateTimerHandle` (`self.TimerHandle`)))

(event `StartFireWeapon`
  (if (not (`self.GetIsDead`))
    (bind _returnvalue (`KismetSystemLibrary.K2_SetTimerDelegate` (delegate `FireAssault`) (`self.FireRate`) true))
    (set `self.TimerHandle` _returnvalue)))

(event `FireAssault`
  (bind _muzzlearrow (`self.MuzzleArrow`))
  (if (> (`self.AmmoInClip`) 20)
    (set `self.IsFiring?` true)
    (`GameplayStatics.SpawnEmitterAttached` (`self.MuzzleEffect`) _muzzlearrow)
    (`GameplayStatics.SpawnSoundAttached` "/Game/Sound/Weapons/SMG_Thompson/Cue_Thompson_Shot.Cue_Thompson_Shot" _muzzlearrow)
    (`|SpawnActorFromClass` "/Game/Bullet_bp.Bullet_bp_C" (`KismetMathLibrary.MakeTransform` (`SceneComponent.K2_GetComponentLocation` _muzzlearrow) (`SceneComponent.K2_GetComponentRotation` _muzzlearrow)) "AlwaysSpawn" "OverrideRootScale" null self)
    (else
      (set `self.IsFiring?` false)
      (`KismetSystemLibrary.PrintString` "empty"))))

(fn `CalcSpread`
  (returns (`Projectil Spawn` :type "Transform Structure"))
  (bind _muzzlearrow (`self.MuzzleArrow`))
  (return (`KismetMathLibrary.MakeTransform` (`SceneComponent.K2_GetComponentLocation` _muzzlearrow) (`KismetMathLibrary.Conv_VectorToRotator` (`KismetMathLibrary.RandomUnitVectorInCone` (`SceneComponent.GetForwardVector` _muzzlearrow) (`self.WeaponSpread`))) (0.0 0.0 0.0))))

(fn `UserConstructionScript`
  (bind _weaponmesh2 (`self.WeaponMesh2`))
  (`|ExecutionSequence`
    (:`then_0`
      (`SceneComponent.K2_AttachToComponent` _weaponmesh2 (`self.Mesh`) "GunSocket" "KeepRelative" "KeepRelative" "KeepRelative" true))
    (:`then_1`
      (`SceneComponent.K2_AttachToComponent` (`self.MuzzleArrow`) _weaponmesh2 "Muzzle" "SnapToTarget" "SnapToTarget" "KeepRelative" true))))