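; Player controller Blueprint that sets up the player's HUD and switches to the death screen when the player dies.
; On BeginPlay it adds PlayerUI_BP to the viewport and binds to the Player_BP pawn's OnDeathRequest dispatcher.
; That event clears all widgets, shows DeathUI_BP and enables the mouse cursor with UI-only input.
; A leftover binding to the game mode's OnDeathRequest is disconnected and never runs.
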(event `self.ReceiveBeginPlay`
  (`|ExecutionSequence`
    (:`then_0`
      (bind _returnvalue (`|CreateWidget` "/Game/UI/PlayerUI_BP.PlayerUI_BP_C"))
      (`UserWidget.AddToViewport` _returnvalue 0))
    (:`then_1`
      (bind _asplayer_bp (cast `/Game/Player/Player_BP` (`GameplayStatics.GetPlayerPawn` 0)))
      (add `PlayerCharacter.OnDeathRequest` _asplayer_bp (delegate `OnDeathRequest_Event_0`)))))

(event `OnDeathRequest_Event_0`
  (bind _returnvalue (`GameplayStatics.GetPlayerController` 0))
  (bind _returnvalue_2 (`|CreateWidget` "/Game/UI/DeathUI_BP.DeathUI_BP_C"))
  (`WidgetLayoutLibrary.RemoveAllWidgets`)
  (`UserWidget.AddToViewport` _returnvalue_2 0)
  (set `PlayerController.bShowMouseCursor` true _returnvalue)
  (`WidgetBlueprintLibrary.SetInputMode_UIOnlyEx` _returnvalue _returnvalue_2))

(fn `UserConstructionScript`)