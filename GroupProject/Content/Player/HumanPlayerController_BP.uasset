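; Player controller for the human player that manages the in-game UI and the game over screen.
; On BeginPlay it adds a player UI widget to the viewport and pre-creates a death UI widget, stored as the game over screen.
; Tick polls the current state of the project's game mode and calls AddToViewport on the stored screen every frame the state is Game Over.
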(event `self.ReceiveBeginPlay`
  ;[1 1 1] Displays the player UI on to the viewport
  (`|ExecutionSequence`
    (:`then_0`
      (bind _returnvalue (`|CreateWidget` "/Game/UI/PlayerUI_BP.PlayerUI_BP_C"))
      (`UserWidget.AddToViewport` _returnvalue 0))
    (:`then_1`
      (bind _returnvalue_2 (`|CreateWidget` "/Game/UI/DeathUI_BP.DeathUI_BP_C"))
      (set `self.GameOverScreen` _returnvalue_2))))

(event `self.ReceiveTick`
  (params (DeltaSeconds :type "Float (single-precision)"))
  (bind _asmy_group_project_game_mode_bp (cast `/Game/MyGroupProjectGameMode_BP` (`GameplayStatics.GetGameMode`)))
  (switch `EGameState` (`GroupProjectGameMode.GetCurrentState` _asmy_group_project_game_mode_bp)
    (:`EGameOver`
      (`UserWidget.AddToViewport` (`self.GameOverScreen`) 0))))

(fn `UserConstructionScript`)